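; BP_P38 is a player-controlled P-38 plane pawn that constantly flies along its forward vector through movement input added every Tick.
; Enhanced Input IA_Move applies frame-rate-scaled local rotation, with X driving roll and Y driving pitch.
; IA_Fire spawns a BP_Roket at the Arrow component's transform, with the plane as owner and instigator.
; Legacy Pitch and Roll axis events remain, but their rotation logic is disconnected.
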(event Input|EnhancedActionEvents|EnhancedInputActionIA_Fire
  (params (ActionValue :type Boolean) (ElapsedSeconds :type Float%20%28double-precision%29) (TriggeredSeconds :type Float%20%28double-precision%29) (InputAction :type Input%20Action%20Object%20Reference :default "/Game/P_38Game/Input/IA_Fire.IA_Fire"))
  (bind _self self)
  (Game|SpawnActorfromClass "/Game/Blueprints/BP_Roket.BP_Roket_C" (Transformation|GetWorldTransform (Variables|Default|GetArrow)) "Undefined" "MultiplyWithRoot" _self _self))

(event Input|EnhancedActionEvents|EnhancedInputActionIA_Move
  (params (ActionValue :type Vector%202D%20Structure) (ElapsedSeconds :type Float%20%28double-precision%29) (TriggeredSeconds :type Float%20%28double-precision%29) (InputAction :type Input%20Action%20Object%20Reference :default "/Game/P_38Game/Input/IA_Move.IA_Move"))
  (Transformation|AddActorLocalRotation (Math|Rotator|MakeRotator (* (.x ActionValue) (Utilities|Time|GetWorldDeltaSeconds) 6e+01) 0.0 0.0) false false)
  (Transformation|AddActorLocalRotation (Math|Rotator|MakeRotator 0.0 (* (.y ActionValue) (Utilities|Time|GetWorldDeltaSeconds) 6e+01) 0.0) false false))

(event EventTick
  (params (DeltaSeconds :type Float%20%28single-precision%29))
  ;[0.15 0.15 0.15 0.5] Move go
  (Pawn|Input|AddMovementInput (Transformation|GetActorForwardVector) 1.0 false))

(event Input|AxisEvents|InputAxisPitch
  (params (AxisValue :type Float%20%28single-precision%29))
  ;[0.15 0.15 0.15 0.5] Pitch
)

(event Input|AxisEvents|InputAxisRoll
  (params (AxisValue :type Float%20%28single-precision%29))
  ;[0.15 0.15 0.15 0.5] Roll
)

(fn ConstructionScript)